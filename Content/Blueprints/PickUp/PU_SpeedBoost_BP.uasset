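; Speed boost pickup that raises the player character's max walk speed when its collection trigger is overlapped, then destroys itself with a sound and particle burst.
; The overlap handler always targets player 0, without checking the overlapping actor.
; It sets a timer on TopDownGameMode to call TimerSpeedBoost, so the callback outlives the pickup.
; The mesh spin timeline is never executed.
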(event `self.ReceiveBeginPlay`)

(event `self.CollectionTrigger.OnComponentBeginOverlap`
  (params (OverlappedComponent :type "PrimitiveComponent Object Reference") (OtherActor :type "Actor Object Reference") (OtherComp :type "PrimitiveComponent Object Reference") (OtherBodyIndex :type Integer) (bFromSweep :type Boolean) (SweepResult :type "HitResult Structure (by ref)"))
  (bind _returnvalue (`self.K2_GetActorLocation`))
  (bind _astop_down_character (cast `/Game/Blueprints/TopDownCharacter` (`GameplayStatics.GetPlayerCharacter` 0)))
  (set `CharacterMovementComponent.MaxWalkSpeed` 900.0 (`Character.CharacterMovement` _astop_down_character))
  (bind _astop_down_game_mode (cast `/Game/Blueprints/TopDownGameMode` (`GameplayStatics.GetGameMode`)))
  (`KismetSystemLibrary.K2_SetTimer` _astop_down_game_mode "TimerSpeedBoost" 5.0)
  (`GameplayStatics.PlaySoundAtLocation` "/Game/Blueprints/PickUp/Audio/Pickup.Pickup" _returnvalue (struct) 1.0 1.0 0.0 null null null) ; Add specific sound
  (`GameplayStatics.SpawnEmitterAtLocation` "/Game/InfinityBladeEffects/Effects/FX_Mobile/ICE/combat/P_Impact_Shield.P_Impact_Shield" _returnvalue) ; Particules
  (`self.K2_DestroyActor`))

(fn `UserConstructionScript`)