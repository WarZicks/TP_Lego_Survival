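; Mana pickup actor that grants a fixed amount of mana when something overlaps its trigger.
; The overlap sets the mana offset on TopDownGameMode and calls AddMana, then plays a sound, spawns a particle effect and destroys the actor.
; The trigger and particle carry health-pickup names, and the overlap does not check which actor entered.
; The mesh spin timeline and player cast are unconnected and never run.
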(event `self.ReceiveBeginPlay`)

(event `self.HealthTrigger.OnComponentBeginOverlap`
  (params (OverlappedComponent :type "PrimitiveComponent Object Reference") (OtherActor :type "Actor Object Reference") (OtherComp :type "PrimitiveComponent Object Reference") (OtherBodyIndex :type Integer) (bFromSweep :type Boolean) (SweepResult :type "HitResult Structure (by ref)"))
  (bind _returnvalue (`self.K2_GetActorLocation`))
  (bind _astop_down_game_mode (cast `/Game/Blueprints/TopDownGameMode` (`GameplayStatics.GetGameMode`)))
  (set `/Game/Blueprints/TopDownGameMode.ManaOffset` 25.0 _astop_down_game_mode)
  (`/Game/Blueprints/TopDownGameMode.AddMana` _astop_down_game_mode)
  (`GameplayStatics.PlaySoundAtLocation` null _returnvalue (struct) 1.0 1.0 0.0 null null null)
  (`GameplayStatics.SpawnEmitterAtLocation` "/Game/InfinityBladeEffects/Effects/FX_Ability/Heal/P_HealthPotion_Pickup_01.P_HealthPotion_Pickup_01" _returnvalue)
  (`self.K2_DestroyActor`))

(fn `UserConstructionScript`)