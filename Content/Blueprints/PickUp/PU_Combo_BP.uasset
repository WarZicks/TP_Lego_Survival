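; Combo pickup Blueprint that reacts when something overlaps its collection trigger.
; On overlap it plays a shield lift sound, spawns an ice shield impact particle at its location and destroys itself, without granting any effect to the overlapping actor.
; A timeline-driven mesh spin and a player character cast are present but unconnected, so they never run.
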(event `self.ReceiveBeginPlay`)

(event `self.CollectionTrigger.OnComponentBeginOverlap`
  (params (OverlappedComponent :type "PrimitiveComponent Object Reference") (OtherActor :type "Actor Object Reference") (OtherComp :type "PrimitiveComponent Object Reference") (OtherBodyIndex :type Integer) (bFromSweep :type Boolean) (SweepResult :type "HitResult Structure (by ref)"))
  (bind _returnvalue (`self.K2_GetActorLocation`))
  (`GameplayStatics.PlaySoundAtLocation` "/Game/Knight/Sounds/Shield_Lift_Cue.Shield_Lift_Cue" _returnvalue (struct) 1.0 1.0 0.0 null null null)
  (`GameplayStatics.SpawnEmitterAtLocation` "/Game/InfinityBladeEffects/Effects/FX_Mobile/Impacts/P_Impact_Shield_Ice.P_Impact_Shield_Ice" _returnvalue)
  (`self.K2_DestroyActor`))

(fn `UserConstructionScript`)