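; Weapon actor Blueprint that deals area damage around itself when TryDealDamage is triggered.
; The event runs a sphere overlap for Pawn objects at the Weapon component's world location, ignoring the owner of the component it is attached to.
; Each overlapped actor receives the passed-in damage through ApplyDamage, with the weapon as damage causer.
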(event `TryDealDamage`
  (params (Damage :type "Float (double-precision)" :default 10.0))
  (bind _outactors (`KismetSystemLibrary.SphereOverlapActors` (`SceneComponent.K2_GetComponentLocation` (`self.Weapon`)) 150.0 (`|MakeArray` "ObjectTypeQuery3" :!type "EObjectTypeQuery Enum") null (`|MakeArray` (`ActorComponent.GetOwner` (`SceneComponent.GetAttachParent` (`self.DefaultSceneRoot`))))))
  (for _array_element _outactors
    (`GameplayStatics.ApplyDamage` _array_element Damage null self)))

(fn `UserConstructionScript`)