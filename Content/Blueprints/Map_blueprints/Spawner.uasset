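; Map spawner actor that periodically spawns random minion and leader AI enemies (Cac, Kamikaze or Range) at its Box transform.
; BeginPlay starts two looping timers: a fixed interval for minions and a random interval, rolled once, for leaders.
; Each spawn is gated by TopDownGameMode's CanSpawn flags, then decrements that mode's matching remaining count and calls its count check.
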(event `SpawnMinion`
  (bind _returnvalue (`SceneComponent.K2_GetComponentToWorld` (`self.Box`)))
  (bind _astop_down_game_mode (cast `/Game/Blueprints/TopDownGameMode` (`GameplayStatics.GetGameMode`)))
  (if (`/Game/Blueprints/TopDownGameMode.CanSpawnMinion` _astop_down_game_mode)
    (switch `int` (`KismetMathLibrary.RandomInteger` 3)
      (:`0`
        (`|SpawnActorFromClass` "/Game/AI/AI_Cac_Character.AI_Cac_Character_C" _returnvalue "AlwaysSpawn" "OverrideRootScale" null null))
      (:`1`
        (`|SpawnActorFromClass` "/Game/AI/AI_Kamikaze_Character.AI_Kamikaze_Character_C" _returnvalue "AlwaysSpawn" "OverrideRootScale" null null))
      (:`2`
        (`|SpawnActorFromClass` "/Game/AI/AI_Range_Character.AI_Range_Character_C" _returnvalue "AlwaysSpawn" "OverrideRootScale" null null)))
    (bind _astop_down_game_mode_2 (cast `/Game/Blueprints/TopDownGameMode` (`GameplayStatics.GetGameMode`)))
    (`/Engine/EditorBlueprintResources/StandardMacros.DecrementInt` (`/Game/Blueprints/TopDownGameMode.MinionCount` _astop_down_game_mode_2)
      (:`  `
        (`/Game/Blueprints/TopDownGameMode.CheckMinionsCount` _astop_down_game_mode_2)))))

(event `self.ReceiveBeginPlay`
  (`|ExecutionSequence`
    (:`then_0`
      (`/Engine/EditorBlueprintResources/StandardMacros.DoOnce` false :!label _label
        (:`Completed`
          (`KismetSystemLibrary.K2_SetTimerDelegate` (delegate `SpawnMinion`) 2.0 true)
          (goto _label :!via `Reset`))))
    (:`then_1`
      (`/Engine/EditorBlueprintResources/StandardMacros.DoOnce` false :!label _label_2
        (:`Completed`
          (`KismetSystemLibrary.K2_SetTimerDelegate` (delegate `SpawnLeader`) (`KismetMathLibrary.RandomFloatInRange` 10.0 30.0) true)
          (goto _label_2 :!via `Reset`))))))

(event `SpawnLeader`
  (bind _returnvalue (`SceneComponent.K2_GetComponentToWorld` (`self.Box`)))
  (bind _astop_down_game_mode (cast `/Game/Blueprints/TopDownGameMode` (`GameplayStatics.GetGameMode`)))
  (if (`/Game/Blueprints/TopDownGameMode.CanSpawnLeader` _astop_down_game_mode)
    (switch `int` (`KismetMathLibrary.RandomInteger` 3)
      (:`0`
        (`|SpawnActorFromClass` "/Game/AI/AI_Cac_Character_Leader.AI_Cac_Character_Leader_C" _returnvalue "AlwaysSpawn" "OverrideRootScale" null null))
      (:`1`
        (`|SpawnActorFromClass` "/Game/AI/AI_Kamikaze_Character_Leader.AI_Kamikaze_Character_Leader_C" _returnvalue "AlwaysSpawn" "OverrideRootScale" null null))
      (:`2`
        (`|SpawnActorFromClass` "/Game/AI/AI_Range_Character_leader.AI_Range_Character_leader_C" _returnvalue "AlwaysSpawn" "OverrideRootScale" null null)))
    (bind _astop_down_game_mode_2 (cast `/Game/Blueprints/TopDownGameMode` (`GameplayStatics.GetGameMode`)))
    (`/Engine/EditorBlueprintResources/StandardMacros.DecrementInt` (`/Game/Blueprints/TopDownGameMode.LeaderCount` _astop_down_game_mode_2)
      (:`  `
        (`/Game/Blueprints/TopDownGameMode.CheckLeaderCount` _astop_down_game_mode_2)))))

(fn `UserConstructionScript`)